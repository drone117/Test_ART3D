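; BP_ColorPicker is an actor attached to a BP_Cube that displays the cube's name and a color, and passes color changes to it.
; BeginPlay creates one dynamic material instance from MI_CubeMaterial, shared by the front and back planes.
; InitColorPicker finds the cube through the root's attach parent, then fills both texts, reading the color from its own material.
; ChangeCubeColor updates that material, the parent cube and the color text.
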(event Custom|InitColorPicker
  ;[1 1 1] Инициализация параметров эктора
  (bind _asbp_cube (Utilities|Casting|CastToBP_Cube (Components|GetOwner (Transformation|GetAttachParent (Variables|Default|GetDefaultSceneRoot)))))
  (bind _output_get (Variables|Default|SetParentCube _asbp_cube))
  (Rendering|Components|TextRender|SetText (Variables|Default|GetCubeName) (Utilities|Text|ToText(String) (Utilities|GetObjectName _output_get)))
  (bind _returnvalue (Rendering|Material|GetVectorParameterValue (Variables|Default|GetDynamicMaterial) "Color" :!class /Script/Engine.MaterialInstanceDynamic))
  (bind _output_get_2 (Variables|Default|SetNewCubeColor _returnvalue))
  (Rendering|Components|TextRender|SetText (Variables|Default|GetCubeColor) (Utilities|Text|ToText(String) _output_get_2)))

(event Custom|ChangeCubeColor
  (params (NewCubeColor :type Linear%20Color%20Structure))
  ;[1 1 1] Изменение параметров цвета эктора и его родительского куба
  (bind _output_get (Variables|Default|SetNewCubeColor NewCubeColor))
  (Rendering|Material|SetVectorParameterValue (Variables|Default|GetDynamicMaterial) "Color" _output_get :!class /Script/Engine.MaterialInstanceDynamic)
  (Default|ChangeCubeColor (Variables|Default|GetParentCube) (Variables|Default|GetNewCubeColor))
  (Rendering|Components|TextRender|SetText (Variables|Default|GetCubeColor) (Utilities|Text|ToText(String) (Variables|Default|GetNewCubeColor))))

(event EventBeginPlay
  ;[1 1 1] Создание динамичного материала для управления в рантайме
  (bind _returnvalue (Rendering|Material|CreateDynamicMaterialInstance "/Game/Materials/MI_CubeMaterial.MI_CubeMaterial" "None" "None" :!class /Script/Engine.KismetMaterialLibrary))
  (Variables|Default|SetDynamicMaterial _returnvalue)
  (Rendering|Material|SetMaterial (Variables|Default|GetPlaneBack) 0 (Variables|Default|GetDynamicMaterial)))

(fn ConstructionScript)