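; BP_Cube is an actor that, on first overlapping a BP_SplineActor tagged "spline", drops physics and loops along its spline.
; A Timeline maps its alpha to spline distance, setting location and tangent-facing rotation each update, and restarts when finished.
; Reaching each expected spline point within a tolerance toggles the Timeline play rate between full and half speed.
; A dynamic material created at BeginPlay lets ChangeCubeColor recolor the cube at runtime.
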(event OnComponentBeginOverlap(StaticMesh)
  (params (OverlappedComponent :type Primitive%20Component%20Object%20Reference) (OtherActor :type Actor%20Object%20Reference) (OtherComp :type Primitive%20Component%20Object%20Reference) (OtherBodyIndex :type Integer) (bFromSweep :type Boolean) (SweepResult :type Hit%20Result%20Structure%20%28by%20ref%29))
  (bind _staticmesh (Variables|Default|GetStaticMesh))
  ;[1 1 1] Проверка оверлапа со SplineActor, у которого изначально выставлен тэг 'spline'. В случае оверлапов с несколькими экторами позволяет избежать ненуженых кастов.
  (if (Actor|ActorHasTag OtherActor "spline")
    (Variables|Default|GetSplineActor
      (:then)
      (:else
        (bind _asbp_spline_actor (Utilities|Casting|CastToBP_SplineActor OtherActor))
        (Variables|Default|SetSplineActor _asbp_spline_actor)
        (Physics|SetSimulatePhysics _staticmesh false)
        (Collision|SetCollisionEnabled _staticmesh "QueryOnly")
        (CallFunction|PlayTimeline)))))

(event Custom|PlayTimeline
  (bind _splineactor (Variables|Default|GetSplineActor))
  (bind _splineactor_2 (Variables|Default|GetSplineActor))
  (bind _spline (Variables|/Game/Blueprints/BP_SplineActor.BP_SplineActor_C|GetSpline _splineactor))
  (bind _spline_2 (Variables|/Game/Blueprints/BP_SplineActor.BP_SplineActor_C|GetSpline _splineactor_2))
  ;[1 1 1] Воспроизведение таймлайна по координатам SplineActor
  (bind _actormovement (Timeline|Timeline PlayFromStart)
    (:Update
      (Transformation|SetActorLocation (Spline|GetLocationatDistanceAlongSpline _spline (Math|Float|Lerp 0.0 (Spline|GetDistanceAlongSplineatSplinePoint _spline_2 (- (Spline|GetNumberOfSplinePoints _spline_2) 1)) _actormovement) "World") false false)
      (Transformation|SetActorRotation (Math|Conversions|RotationFromXVector (Spline|GetTangentatDistanceAlongSpline _spline (Math|Float|Lerp 0.0 (Spline|GetDistanceAlongSplineatSplinePoint _spline_2 (- (Spline|GetNumberOfSplinePoints _spline_2) 1)) _actormovement) "World")))
      ;;[1 1 1] Проверка, что текущая позиция куба соответсвует точке сплайна
      (if (Utilities|Operators|EqualEqual (Transformation|GetActorLocation) (Spline|GetLocationatSplinePoint (Variables|/Game/Blueprints/BP_SplineActor.BP_SplineActor_C|GetSpline (Variables|Default|GetSplineActor)) (Variables|Default|GetPoint%20Index) "World") 5.0)
        ;;[1 1 1] В случае, если точка чётная, снижение скорости в 2 раза
        (if (Variables|Default|GetbCrossedSlowingPoint?)
          (Variables|Default|SetPlayRate 1e+01)
          (else
            (Variables|Default|SetPlayRate 5.0)))
        (bind _result (Math|Integer|IncrementInt (Variables|Default|GetPoint%20Index))
          (:%20%20
            (Components|Timeline|SetPlayRate (Variables|Default|GetTimeline) (/ 1.0 (Variables|Default|GetPlayRate)))
            (Variables|Default|SetbCrossedSlowingPoint? (not (Variables|Default|GetbCrossedSlowingPoint?)))
            (if (== _result (- (Spline|GetNumberOfSplinePoints (Variables|/Game/Blueprints/BP_SplineActor.BP_SplineActor_C|GetSpline (Variables|Default|GetSplineActor))) 1))
              (Variables|Default|SetPoint%20Index 0))))))
    (:Finished
      (CallFunction|PlayTimeline))))

(event Custom|ChangeCubeColor
  (params (NewColor :type Linear%20Color%20Structure))
  ;[1 1 1] Изменение цвета куба
  (Rendering|Material|SetVectorParameterValue (Variables|Default|GetDynamicCubeMaterial) "Color" NewColor :!class /Script/Engine.MaterialInstanceDynamic))

(event EventBeginPlay
  (Components|Timeline|SetPlayRate (Variables|Default|GetTimeline) (/ 1.0 (Variables|Default|GetPlayRate)))
  ;[1 1 1] Создание динамичного материала для управление цветом в рантайме
  (bind _returnvalue (Rendering|Material|CreateDynamicMaterialInstance "/Game/Materials/MI_CubeMaterial.MI_CubeMaterial" "None" "None" :!class /Script/Engine.KismetMaterialLibrary))
  (Variables|Default|SetDynamicCubeMaterial _returnvalue)
  (Rendering|Material|SetMaterial (Variables|Default|GetStaticMesh) 0 (Variables|Default|GetDynamicCubeMaterial)))

(fn ConstructionScript)