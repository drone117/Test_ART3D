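; Game mode that runs a day-night cycle and manages colorable cubes.
; A looping timer pitches the level's DirectionalLight (spawned if missing) at a rate derived from DayLength, with DoOnce gates switching all SpotLights at half-cycle thresholds and resetting each full turn.
; Cube events spawn a BP_Cube with an attached BP_ColorPicker, track pairs in an array and map, and remove or recolor them by index.
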(event Custom|DayNightCycle
  (bind _output_get (Variables|Default|SetLightRotation (+ (Variables|Default|GetLightRotation) (/ 3.6e+02 (* (Variables|Default|GetDayLength) 86.4)))))
  (Transformation|SetActorRelativeRotation (Variables|Default|GetDirectionalLight) (Math|Rotator|MakeRotator 0.0 _output_get 0.0))
  ;[1 1 1] Проверка текущего поворота солнца и вызов единовременный вызов функции SwitchLights, который сбрасывается при полном прохождении небосвода
  (Utilities|FlowControl|Sequence
    (:then_0
      (if (and (>= (Variables|Default|GetLightRotation) 1.8e+02) (< (Variables|Default|GetLightRotation) 3.6e+02))
        (Utilities|FlowControl|DoOnce false :!label _label
          (:Completed
            (CallFunction|SwitchLights 0.0)))
        (else
          (Utilities|FlowControl|DoOnce false :!label _label_2
            (:Completed
              (CallFunction|SwitchLights 8.0))))))
    (:then_1
      (if (>= (Variables|Default|GetLightRotation) 3.6e+02)
        (Variables|Default|SetLightRotation 0.0)
        (Utilities|FlowControl|Sequence
          (:then_0
            (goto _label Reset))
          (:then_1
            (goto _label_2 Reset)))))))

(event Custom|SwitchLights
  (params (NewIntensity :type Float%20%28single-precision%29))
  ;[1 1 1] Отключение/включение светильников
  (for _array_element (Variables|Default|GetLights)
    (Rendering|Components|Light|SetIntensity (Variables|/Script/Engine.Light|GetLightComponent _array_element) NewIntensity)))

(event Custom|SpawnCube
  (bind _cubetransform (Variables|Default|GetCubeTransform))
  ;[1 1 1] Создание куба, присоединение ColorPicker к нему и инициалищация ColorPicker
  (bind _returnvalue (Game|SpawnActorfromClass "/Game/Blueprints/BP_Cube.BP_Cube_C" (Variables|Default|GetCubeTransform) "Undefined" "MultiplyWithRoot" 0 0))
  (Variables|Default|SetCurrentCube _returnvalue)
  (bind _returnvalue_2 (Game|SpawnActorfromClass "/Game/Blueprints/BP_ColorPicker.BP_ColorPicker_C" (Math|Transform|MakeTransform (+ (.location _cubetransform) "0.000000,0.000000,100.000000") (.rotation _cubetransform) (.scale _cubetransform)) "Undefined" "MultiplyWithRoot" 0 0))
  (bind _output_get (Variables|Default|SetCurrentColorPicker _returnvalue_2))
  (Transformation|AttachActorToActor _output_get (Variables|Default|GetCurrentCube) "None" "KeepWorld" "KeepWorld" "KeepWorld" true)
  (Utilities|Map|Add (Variables|Default|GetCubesPickersMap) (Variables|Default|GetCurrentCube) (Variables|Default|GetCurrentColorPicker))
  (Utilities|Array|Add (Variables|Default|GetCubesArray) (Variables|Default|GetCurrentCube))
  (Default|InitColorPicker (Variables|Default|GetCurrentColorPicker)))

(event Custom|StartCycle
  (Variables|Default|GetDirectionalLight
    (:then
      _)
    (:else
      (bind _returnvalue (Game|SpawnActorfromClass "/Script/Engine.DirectionalLight" (Math|Transform|MakeTransform "0, 0, 0" "0, 0, 0" "1.000000,1.000000,1.000000") "Undefined" "MultiplyWithRoot" 0 0))
      (Variables|Default|SetDirectionalLight _returnvalue)))
  ;[1 1 1] Таймер для реализации цикла
  (bind _returnvalue_2 (Utilities|Time|SetTimerbyEvent (delegate Custom|DayNightCycle) (/ 1.0 (Variables|Default|GetTimerSmoothness)) true))
  (Variables|Default|SetTimerHandle _returnvalue_2))

(event Custom|RemoveCube
  (params (CubeIndex :type Integer))
  (bind _cubesarray (Variables|Default|GetCubesArray))
  (bind _output (Utilities|Array|Get(acopy) _cubesarray CubeIndex))
  ;[1 1 1] Удаление куба и ColorPicker
  (Actor|DestroyActor (.Value (Utilities|Map|Find (Variables|Default|GetCubesPickersMap) _output)))
  (Actor|DestroyActor _output)
  (Utilities|Array|RemoveIndex _cubesarray CubeIndex))

(event Custom|ChangeColor
  (params (SelectedColor :type Linear%20Color%20Structure) (CubeIndex :type Integer))
  ;[1 1 1] Изменение цвета через BP_ColorPicker
  (Default|ChangeCubeColor (.Value (Utilities|Map|Find (Variables|Default|GetCubesPickersMap) (Utilities|Array|Get(acopy) (Variables|Default|GetCubesArray) CubeIndex))) SelectedColor))

(event Custom|SetDayLength
  (params (NewLength :type Float%20%28double-precision%29))
  ;[1 1 1] Изменение длины дня
  (Variables|Default|SetDayLength NewLength))

(event EventBeginPlay
  ;[1 1 1] Получение экторов DirectionalLight и светильников SpotLight, размещенных на уровне и запуск цикла дня и ночи
  (bind _returnvalue (Actor|GetActorOfClass "/Script/Engine.DirectionalLight"))
  (Variables|Default|SetDirectionalLight _returnvalue)
  (bind _outactors (Actor|GetAllActorsOfClass "/Script/Engine.SpotLight"))
  (Variables|Default|SetLights _outactors)
  (CallFunction|StartCycle))

(fn ConstructionScript)

(fn GetCurrentCubeDisplayName
  (bind _currentcube (Variables|Default|GetCurrentCube)
    (:then
      (return (Utilities|GetDisplayName _currentcube)))
    (:else
      (return ""))))